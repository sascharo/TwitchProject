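; Player character Blueprint handling movement, sprinting and left/right melee attacks.
; Axis input moves the character relative to controller yaw, Left Shift toggles walk speed while held, and mouse buttons play sections of the mutant attack montage.
; The MoveForward axis event also smooths PlayerLeanAmount toward CalcLeanAmount's target.
; That target follows turn input while sprinting on the ground, otherwise easing back to upright faster.
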(event EventBeginPlay)

(event Collision|EventActorBeginOverlap
  (params (OtherActor :type Actor%20Object%20Reference)))

(event EventTick
  (params (DeltaSeconds :type Float%20%28single-precision%29)))

(event Input|AxisEvents|InputAxisMoveForward
  (params (AxisValue :type Float%20%28single-precision%29))
  (bind (_leanamount _interpolatedspeed) (CallFunction|CalcLeanAmount))
  (Pawn|Input|AddMovementInput (Math|Vector|GetForwardVector (Math|Rotator|MakeRotator 0.0 0.0 (.Yaw (Math|Rotator|BreakRotator (Pawn|GetControlRotation :!class /Script/Engine.Pawn))))) AxisValue false)
  (Variables|Default|SetPlayerLeanAmount (Math|Interpolation|FInterpTo (Variables|Default|GetPlayerLeanAmount) _leanamount (Utilities|Time|GetWorldDeltaSeconds) _interpolatedspeed)))

(event Input|AxisEvents|InputAxisMoveRight
  (params (AxisValue :type Float%20%28single-precision%29))
  (Pawn|Input|AddMovementInput (Math|Vector|GetRightVector (Math|Rotator|MakeRotator 0.0 0.0 (.Yaw (Math|Rotator|BreakRotator (Pawn|GetControlRotation :!class /Script/Engine.Pawn))))) AxisValue false))

(event Input|KeyboardEvents|LeftShift
  (params (Key :type Key%20Structure :default "None"))
  (bind _charactermovement (Variables|Character|GetCharacterMovement))
  (:Pressed
    (Variables|/Script/Engine.CharacterMovementComponent|SetMaxWalkSpeed _charactermovement 2.2e+02)
    (Variables|Default|SetisSprinting? true))
  (:Released
    (Variables|/Script/Engine.CharacterMovementComponent|SetMaxWalkSpeed _charactermovement 1.1e+02)
    (Variables|Default|SetisSprinting? false)))

(event Input|MouseEvents|LeftMouseButton
  (params (Key :type Key%20Structure :default "None"))
  (:Pressed
    (Animation|PlayAnimMontage "/Game/Mutant/Animations/Montage_MutantAttack.Montage_MutantAttack" 1.0 "LeftAttack")))

(event Input|MouseEvents|RightMouseButton
  (params (Key :type Key%20Structure :default "None"))
  (:Pressed
    (Animation|PlayAnimMontage "/Game/Mutant/Animations/Montage_MutantAttack.Montage_MutantAttack" 1.0 "RightAttack")))

(fn ConstructionScript)

(fn CalcLeanAmount
  (bind _issprinting_ (Variables|Default|GetisSprinting?))
  (bind _charactermovement (Variables|Character|GetCharacterMovement))
  (bind _returnvalue (AI|Components|NavMovement|IsFalling _charactermovement))
  (bind _returnvalue_2 (not _issprinting_))
  (bind _returnvalue_3 (or _returnvalue _returnvalue_2))
  (return (select _returnvalue_3 0.0 (Math|Float|Clamp(Float) (Input|AxisValues|GetTurn) -1.0 1.0)) (select _returnvalue_3 1e+01 1.0)))